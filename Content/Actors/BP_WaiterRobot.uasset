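; BP_WaiterRobot is a waiter robot actor that travels continuously along a spline path.
; Tick advances the distance along the spline by Speed times delta time, resetting it to zero once it passes the spline's length.
; Move places the Character component at that point in local space, keeping its scale and building its rotation with the Y axis along the spline's forward direction and Z along its up.
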(event EventTick
  (params (DeltaSeconds :type Float%20%28single-precision%29))
  (Utilities|FlowControl|Sequence
    (:then_0
      (if (> (Variables|Default|GetDistance%20Along%20Spline) (Spline|GetSplineLength (Variables|Default|GetSpline)))
        (Variables|Default|SetDistance%20Along%20Spline 0.0)))
    (:then_1
      (bind _output_get (Variables|Default|SetDistance%20Along%20Spline (+ (* DeltaSeconds (Variables|Default|GetSpeed)) (Variables|Default|GetDistance%20Along%20Spline))))
      (CallFunction|Move _output_get))))

(fn ConstructionScript)

(fn Move
  (params (distance :type Float%20%28double-precision%29))
  (bind _spline (Variables|Default|GetSpline))
  (bind _returnvalue (Spline|GetTransformatDistanceAlongSpline _spline distance "Local" false))
  (Transformation|SetRelativeTransform (Variables|Default|GetCharacter) (Math|Transform|MakeTransform (.location _returnvalue) (Class|KismetMathLibrary|MakeRotfromYZ (Math|Vector|GetForwardVector (.rotation _returnvalue)) (Math|Vector|GetUpVector (.rotation _returnvalue))) (Variables|/Script/Engine.SceneComponent|GetRelativeScale3D (Variables|Default|GetCharacter))) false false))