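; BP_Waitress1 is a legacy waitress actor that moves its Character component along a spline.
; Each Tick advances a distance by Speed and delta time, then applies the spline's local-space transform at that distance, keeping the component's scale.
; Rotation maps the spline's forward vector to the component's Y axis and keeps spline up as Z, suiting a Y-forward mesh.
; The distance has no wrap or end check in the graph.
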(event EventTick
  (params (DeltaSeconds :type Float%20%28single-precision%29))
  (Variables|Default|SetDistance%20Along%20Spline (+ (* DeltaSeconds (Variables|Default|GetSpeed)) (Variables|Default|GetDistance%20Along%20Spline)))
  (Transformation|SetRelativeTransform (Variables|Default|GetCharacter) (Math|Transform|MakeTransform (.location (Spline|GetTransformatDistanceAlongSpline (Variables|Default|GetSpline) (Variables|Default|GetDistance%20Along%20Spline) "Local" false)) (Class|KismetMathLibrary|MakeRotfromYZ (Math|Vector|GetForwardVector (.rotation (Spline|GetTransformatDistanceAlongSpline (Variables|Default|GetSpline) (Variables|Default|GetDistance%20Along%20Spline) "Local" false))) (Math|Vector|GetUpVector (.rotation (Spline|GetTransformatDistanceAlongSpline (Variables|Default|GetSpline) (Variables|Default|GetDistance%20Along%20Spline) "Local" false)))) (Variables|/Script/Engine.SceneComponent|GetRelativeScale3D (Variables|Default|GetCharacter))) false false))

(fn ConstructionScript)