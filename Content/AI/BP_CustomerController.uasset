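; BP_CustomerController is the AI controller for customers, running the BT_Customer behavior tree on BeginPlay.
; A fast looping timer polls the blackboard's CustomerState enum.
; As written, it broadcasts ChangeCustomerState whenever that value equals the cached state, rather than when it differs, so real changes are never copied.
; Unconnected nodes for setting TargetTable or TargetCashier with a matching state never run.
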(event EventBeginPlay
  (AI|RunBehaviorTree "/Game/AI/BT_Customer.BT_Customer")
  (Utilities|Time|SetTimerbyFunctionName 0 "UpdateCustomerState" 0.01 true))

(fn ConstructionScript)

(fn UpdateCustomerState
  (bind _returnvalue (Utilities|Name|MakeLiteralName "CustomerState"))
  (bind _returnvalue_2 (AI|GetBlackboard 0))
  (bind _returnvalue_3 (Class|BlackboardComponent|GetValueasEnum _returnvalue_2 _returnvalue))
  (bind _returnvalue_4 (Utilities|Enum|ByteToEnumEN_CustomerState _returnvalue_3))
  (if (Utilities|Enum|Equal(Enum) _returnvalue_4 (Variables|Default|GetCustomerState))
    (bind _output_get (Variables|Default|SetCustomerState _returnvalue_4))
    (Default|CallEventDispatcherChangeCustomerState _output_get)))