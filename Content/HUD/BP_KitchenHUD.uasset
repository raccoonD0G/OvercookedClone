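; HUD Blueprint that creates the kitchen widget for the owning player and adds it to the viewport on BeginPlay.
; InitKitchenWidget passes the FinishStation reference to the widget's Init.
; While that reference is not valid, it retries itself through a short function-name timer, so the widget can appear before it is initialized.
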(event EventBeginPlay
  (bind _returnvalue (UserInterface|CreateWidget (Variables|Default|GetKitchenWidgetClass) (Game|Player|GetOwningPlayerController)))
  (bind _output_get (Variables|Default|SetKitchenWidget _returnvalue))
  (CallFunction|InitKitchenWidget)
  (UserInterface|Viewport|AddtoViewport _output_get 0))

(event Collision|EventActorBeginOverlap
  (params (OtherActor :type Actor%20Object%20Reference)))

(event EventTick
  (params (DeltaSeconds :type Float%20%28single-precision%29)))

(fn ConstructionScript)

(fn InitKitchenWidget
  (Utilities|IsValid (Variables|Default|GetFinishStation)
    (:Is%20Valid
      (Class|KitchenWidget|Init (Variables|Default|GetKitchenWidget) (Variables|Default|GetFinishStation)))
    (:Is%20Not%20Valid
      (Utilities|Time|SetTimerbyFunctionName 0 "InitKitchenWidget" 0.1))))